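; Boss encounter trigger actor that tracks the current phase of an in-game boss fight.
; Overlapping its EnemyTrigger component sets the phase to 1, and pressing C increments it through player input enabled at BeginPlay.
; The phase value is only stored here, and a view-target switch to this actor is left unconnected.
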(event OnComponentBeginOverlap(EnemyTrigger)
  (params (OtherActor :type Actor%20Object%20Reference) (OtherComp :type Primitive%20Component%20Object%20Reference) (OtherBodyIndex :type Integer) (bFromSweep :type Boolean) (SweepResult :type Hit%20Result%20Structure%20%28by%20ref%29))
  (Variables|Default|SetCurrentPhase 1))

(event EventBeginPlay
  (Input|EnableInput (Game|GetPlayerController 0)))

(event Input|KeyboardEvents|C
  (:Pressed
    (Variables|Default|SetCurrentPhase (+ (Variables|Default|GetCurrentPhase) 1))))

(fn ConstructionScript)