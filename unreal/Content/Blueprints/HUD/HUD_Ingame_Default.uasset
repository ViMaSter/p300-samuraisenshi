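; In-game HUD that shows an Aim widget following the player character on screen and pointing in the attack direction.
; After a short startup delay it creates the Aim UMG widget and adds it to the viewport at a high Z-order.
; DrawHUD repositions it at the character's projected screen location with a vertical offset.
; Tick converts the player controller's AttackDirectionAxis into degrees to set the widget's direction and store the angle.
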(event EventBeginPlay
  (Utilities|FlowControl|Sequence
    (:then_0
      (Utilities|FlowControl|Delay 0 1.0)
      ;[1 1 1] Construct UMG-widgets
      ;;[1 1 1] AimWidget
      (bind _returnvalue (UserInterface|CreateWidget "/Game/Blueprints/HUD/Widgets/Aim.Aim_C"))
      (Variables|Default|SetAimWidgetConstructed _returnvalue)
      (Class|UserWidget|SetZOrderinViewport (Variables|Default|GetAimWidgetConstructed) 2000)
      (Utilities|FlowControl|Delay 0)
      (UserInterface|Viewport|AddtoViewport (Variables|Default|GetAimWidgetConstructed)))))

(event EventTick
  (params (DeltaSeconds :type Float%20%28single-precision%29))
  (Utilities|FlowControl|Sequence
    (:then_0
      ;[1 1 1] Run UMG-widgets functions
      ;;[1 1 1] AimWidget
      (bind _aspc_ingame_default_c (Utilities|Casting|CastToPC_Ingame_Default (Game|Player|GetOwningPlayerController)))
      (bind _asaim_c (Utilities|Casting|CastToAim (Variables|Default|GetAimWidgetConstructed)))
      (Default|SetDirection _asaim_c (Class|KismetMathLibrary|DegAtan2 (.X (Math|Vector2D|BreakVector2D (Variables|/Game/Blueprints/PlayerController/PC_Ingame_Default.PC_Ingame_Default_C|GetattackDirectionAxis _aspc_ingame_default_c))) (.Y (Math|Vector2D|BreakVector2D (Variables|/Game/Blueprints/PlayerController/PC_Ingame_Default.PC_Ingame_Default_C|GetattackDirectionAxis _aspc_ingame_default_c)))))
      (Variables|Default|SetlookingAtInDegree (Class|KismetMathLibrary|DegAtan2 (.X (Math|Vector2D|BreakVector2D (Variables|/Game/Blueprints/PlayerController/PC_Ingame_Default.PC_Ingame_Default_C|GetattackDirectionAxis _aspc_ingame_default_c))) (.Y (Math|Vector2D|BreakVector2D (Variables|/Game/Blueprints/PlayerController/PC_Ingame_Default.PC_Ingame_Default_C|GetattackDirectionAxis _aspc_ingame_default_c))))))))

(event EventDrawHUD
  (params (SizeX :type Integer) (SizeY :type Integer))
  (bind _returnvalue (Game|GetPlayerCharacter 0))
  (bind _returnvalue_2 (Transformation|GetActorLocation _returnvalue))
  (bind _returnvalue_3 (Class|HUD|Project _returnvalue_2))
  (bind (_x _y) (Math|Vector|BreakVector _returnvalue_3))
  (Utilities|FlowControl|Sequence
    (:then_0
      ;[1 1 1] Update UMG-widgets properties
      ;;[1 1 1] AimWidget
      (Class|UserWidget|SetPositioninViewport (Variables|Default|GetAimWidgetConstructed) (Math|Vector2D|MakeVector2D (+ _x 0.0) (+ _y (Variables|Default|GetAimOffsetY)))))))

(fn ConstructionScript)