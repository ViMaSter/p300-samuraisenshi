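; Particle enemy character that sways side to side while steadily descending, hurting the player and taking damage.
; Tick sets its location directly from time since spawn, using a sine wave on Y, fixed X and linearly falling Z, without sweeping.
; Sphere overlaps with a C_Ingame_Default component tagged Hitbox apply damage from CharacterAttributes.
; Incoming damage lowers health through CharacterAttributes and destroys the actor at zero or below, with debug prints.
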(event OnComponentBeginOverlap(Sphere)
  (params (OtherActor :type Actor%20Object%20Reference) (OtherComp :type Primitive%20Component%20Object%20Reference) (OtherBodyIndex :type Integer) (bFromSweep :type Boolean) (SweepResult :type Hit%20Result%20Structure%20%28by%20ref%29))
  (bind _returnvalue (Game|GetPlayerController 0))
  ;[1 1 1] Applying damage
  (Utilities|Casting|CastToC_Ingame_Default OtherActor)
  (if (Utilities|Array|ContainsItem (Variables|/Script/Engine.ActorComponent|GetComponentTags OtherComp) "Hitbox")
    (Development|PrintString "Hitbox")
    (bind _returnvalue_2 (Class|ComponentCharacterAttributes|GetCurrentRegularDamage (Variables|Default|GetCharacterAttributes)))
    (Game|Damage|ApplyDamage OtherActor (Math|Conversions|ToFloat(Integer) _returnvalue_2) _returnvalue _returnvalue "/Script/samuraisenshi.Damage_General")
    (else
      (Development|PrintString "NoHitbox"))))

(event EventTick
  (params (DeltaSeconds :type Float%20%28single-precision%29))
  (bind _returnvalue (Utilities|Time|GetGameTimeinSeconds))
  (bind _spawnedat (Variables|Default|GetspawnedAt))
  (bind _returnvalue_2 (- _returnvalue _spawnedat))
  ;[1 1 1] Sinus movement
  (Transformation|SetActorLocation (Math|Vector|MakeVector 1.2e+03 (* (Math|Trig|Sin(Radians) _returnvalue_2) 2e+02) (- 2.5e+02 (* _returnvalue_2 2e+01))) false))

(event EventAnyDamage
  (params (Damage :type Float%20%28single-precision%29) (DamageType :type Damage%20Type%20Object%20Reference) (InstigatedBy :type Controller%20Object%20Reference) (DamageCauser :type Actor%20Object%20Reference))
  ;[1 1 1] Get damage
  (bind _returnvalue (Class|ComponentCharacterAttributes|SetRegularHealth (Variables|Default|GetCharacterAttributes) (Math|Float|Floor (* -1.0 Damage)) true))
  ;[1 1 1] Check if death
  (if (> _returnvalue 0)
    (Development|PrintString (Utilities|String|BuildString(Integer) "Enemy: Still Alive" "(" _returnvalue ")"))
    (else
      (Development|PrintString (Utilities|String|BuildString(Integer) "Enemy: Dead" "(" _returnvalue ")"))
      (Actor|DestroyActor))))

(event EventBeginPlay
  ;[1 1 1] Sinus movement
  (Variables|Default|SetspawnedAt (Utilities|Time|GetGameTimeinSeconds)))

(fn ConstructionScript
  (|CallParentFunction))