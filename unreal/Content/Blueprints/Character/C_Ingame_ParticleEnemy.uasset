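; Enemy actor that sweeps side to side in a sine wave while steadily descending from its spawn time, at fixed world coordinates.
; Tick computes the position from elapsed time and sets it without sweep.
; Sphere overlap with C_Ingame_Default calls ApplyDamage using the CharacterAttributes regular damage and player controller 0, but sets no damaged actor.
; Received damage and overlaps only print debug strings, with no health or death handling.
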(event OnComponentBeginOverlap(Sphere)
  (params (OtherActor :type Actor%20Object%20Reference) (OtherComp :type Primitive%20Component%20Object%20Reference) (OtherBodyIndex :type Integer) (bFromSweep :type Boolean) (SweepResult :type Hit%20Result%20Structure%20%28by%20ref%29))
  (bind _returnvalue (Game|GetPlayerController 0))
  ;[1 1 1] Applying damage
  (Utilities|Casting|CastToC_Ingame_Default OtherActor)
  (bind _returnvalue_2 (Class|ComponentCharacterAttributes|GetCurrentRegularDamage (Variables|Default|GetCharacterAttributes)))
  (Game|Damage|ApplyDamage 0 (Math|Conversions|ToFloat(Integer) _returnvalue_2) _returnvalue _returnvalue)
  (Development|PrintString 0 (Utilities|String|Append "Enemy hit player" (Utilities|GetDisplayName OtherActor))))

(event EventActorBeginOverlap
  (params (OtherActor :type Actor%20Object%20Reference))
  ;[1 1 1] Applying damage
  (Development|PrintString 0 (Utilities|GetDisplayName OtherActor)))

(event EventTick
  (params (DeltaSeconds :type Float%20%28single-precision%29))
  (bind _returnvalue (Utilities|Time|GetGameTimeinSeconds))
  (bind _spawnedat (Variables|Default|GetspawnedAt))
  (bind _returnvalue_2 (- _returnvalue _spawnedat))
  ;[1 1 1] Sinus movement
  (Transformation|SetActorLocation (Math|Vector|MakeVector 1.2e+03 (* (Math|Trig|Sin(Radians) _returnvalue_2) 2e+02) (- 2.5e+02 (* _returnvalue_2 2e+01))) false))

(event EventAnyDamage
  (params (Damage :type Float%20%28single-precision%29) (DamageType :type Damage%20Type%20Object%20Reference) (InstigatedBy :type Controller%20Object%20Reference) (DamageCauser :type Actor%20Object%20Reference))
  (Development|PrintString 0 (Utilities|String|Append "Enemy got hit by Player: " (Utilities|String|BuildString(Float) (Utilities|GetDisplayName DamageType) " (" Damage ")"))))

(event EventBeginPlay
  ;[1 1 1] Sinus movement
  (Variables|Default|SetspawnedAt (Utilities|Time|GetGameTimeinSeconds)))

(fn ConstructionScript)