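; Default in-game player character, handling a teasing follow camera and an aimed melee attack.
; Each tick offsets the camera boom by facing yaw and Y velocity, ramped by walking time, and rotates the attack pivot to the HUD's look angle.
; Attack input briefly enables the trigger, which damages overlapped particle enemies using CharacterAttributes.
; The E key spawns a particle enemy at a fixed location.
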(event OnComponentBeginOverlap(AttackTrigger)
  (params (OtherActor :type Actor%20Object%20Reference) (OtherComp :type Primitive%20Component%20Object%20Reference) (OtherBodyIndex :type Integer) (bFromSweep :type Boolean) (SweepResult :type Hit%20Result%20Structure%20%28by%20ref%29))
  ;[1 0 0] Attack
  ;;[1 1 1] Applying damage
  (bind _asc_ingame_particleenemy_c (Utilities|Casting|CastToC_Ingame_ParticleEnemy OtherActor))
  (if (Variables|Default|GetAttack_CurrentlyAttacking)
    (Utilities|FlowControl|Sequence
      (:then_0
        (bind _returnvalue (Class|CharacterAttributesComponent|GetCurrentRegularDamage (Variables|Default|GetCharacterAttributes)))
        (Game|Damage|ApplyDamage _asc_ingame_particleenemy_c (Math|Conversions|ToFloat(Integer) _returnvalue) (Game|GetPlayerController 0) (Variables|/Script/Engine.ChildActorComponent|GetChildActor (Variables|Default|GetWeapon)) "/Script/samuraisenshi.GeneralDamage")
        (Development|PrintString 0 (Utilities|String|Append "Player attacks enemy: " (Utilities|GetDisplayName OtherActor)))))))

(event EventTick
  (params (DeltaSeconds :type Float%20%28single-precision%29))
  (bind _attacktrigger (Variables|PlayerAttack|GetAttackTrigger))
  (bind _attack_currentlyattacking (Variables|Default|GetAttack_CurrentlyAttacking))
  (bind _attackpivot (Variables|Default|GetAttackPivot))
  (Utilities|FlowControl|Sequence
    (:then_0
      ;[0 0.753 1] Camera (teasing camera movement)
      (Utilities|FlowControl|Sequence
        (:then_0
          (Variables|Default|SetCamera_UsedVelocity (Variables|/Script/Engine.MovementComponent|GetVelocity (Variables|Character|GetCharacterMovement))))
        (:then_1
          ;;[1 1 1] Check if the player is walking
          (if (!= (.Y (Math|Vector|BreakVector (Variables|/Script/Engine.MovementComponent|GetVelocity (Variables|Character|GetCharacterMovement)))) 0.0)
            ;;[1 1 1] Find out how long the player is walking
            (if (< (Variables|Default|GetCamera_WalkingSince) 0.0)
              (Variables|Default|SetCamera_WalkingSince (Utilities|Time|GetRealTimeSeconds)))
            (else
              (Variables|Default|SetCamera_WalkingSince -1.0)))
          ;;[1 1 1] Consider direction of player
          (Variables|/Script/Engine.SpringArmComponent|SetTargetOffset (Variables|Default|GetCameraBoom) (+ (* (Variables|Default|GetCamera_GeneralOffset) (/ (.Yaw (Class|KismetMathLibrary|BreakRot (Variables|/Script/Engine.SceneComponent|GetRelativeRotation (Variables|Character|GetMesh)))) -9e+01)) (Math|Vector|MakeVector 0.0 (* (* (.Y (Math|Vector|BreakVector (Variables|Default|GetCamera_UsedVelocity))) (* (Variables|Default|GetCamera_MovementIntensity) 0.3)) (Math|Float|Min(Float) (/ (- (Utilities|Time|GetRealTimeSeconds) (Variables|Default|GetCamera_WalkingSince)) (Variables|Default|GetCamera_FullSpeedAfter)) 1.0)) 0.0))))
        (:then_2
          ;[1 0 0] Attack
          ;;[1 1 1] Rotate attack-trigger
          (bind _ashud_ingame_default_c (Utilities|Casting|CastToHUD_Ingame_Default (HUD|GetHUD (Game|GetPlayerController 0)) :!label _label))
          (Transformation|SetRelativeRotation _attackpivot (Class|KismetMathLibrary|MakeRot (+ (Variables|/Game/Blueprints/HUD/HUD_Ingame_Default.HUD_Ingame_Default_C|GetlookingAtInDegree _ashud_ingame_default_c) 9e+01) 9e+01 0.0) false)
          (Variables|/Script/Engine.SceneComponent|SetbAbsoluteRotation _attackpivot true))))
    (:then_1
      (Utilities|FlowControl|Sequence
        (:then_0
          (goto _label))
        (:then_1
          ;;[1 1 1] Toggle attack-state
          (Rendering|SetVisibility _attacktrigger _attack_currentlyattacking false)
          (Variables|/Script/Engine.PrimitiveComponent|SetbGenerateOverlapEvents _attacktrigger _attack_currentlyattacking))))))

(event EventBeginPlay
  ;[0 0.753 1] Camera (teasing camera movement)
  ;;[1 1 1] Reset values we can't hide from defaults
  (Variables|Default|SetCamera_WalkingSince -1.0)
  (Variables|Default|SetCamera_UsedVelocity "0, 0, 0")
  (Input|EnableInput 0))

(event Input|ActionEvents|InputActionAttack
  ;[1 0 0] Attack
  ;;[1 1 1] Toggle attack-state
  (:Pressed
    (Variables|Default|SetAttack_CurrentlyAttacking true)
    (Utilities|FlowControl|Delay 0)
    (Variables|Default|SetAttack_CurrentlyAttacking false)))

(event Input|KeyboardEvents|E
  (:Pressed
    (Game|SpawnActorfromClass "/Game/Blueprints/Character/C_Ingame_ParticleEnemy.C_Ingame_ParticleEnemy_C" (Math|Transform|MakeTransform "1000.000000,1000.000000,100.000000") false 0)))

(fn ConstructionScript)